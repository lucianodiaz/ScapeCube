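; Map creator data holder that keeps the list of obstacles placed in the map creator and a flag for whether the map is a creator map.
; Events add and remove entries in ObstaclesSaved, and getters expose that list and the flag.
; UpdateObstacle finds entries referencing the given obstacle and reapplies that actor's own location and rotation to it, leaving the stored entries unmodified.
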(event `/Game/Blueprints/GameTools/MapCreator/BP_InstanceInterface.AddNewObject`
  (params (NewObject :type "CObstacle Object Reference"))
  (`KismetArrayLibrary.Array_Add` (`self.ObstaclesSaved`) (make `/Game/Blueprints/GameTools/MapCreator/F_SaveData` NewObject)))

(event `/Game/Blueprints/GameTools/MapCreator/BP_InstanceInterface.RemoveObject`
  (params (OldObstacle :type "/Game/Blueprints/GameTools/MapCreator/F_SaveData Structure"))
  (`KismetArrayLibrary.Array_RemoveItem` (`self.ObstaclesSaved`) OldObstacle))

(event `/Game/Blueprints/GameTools/MapCreator/BP_InstanceInterface.UpdateObstacle`
  (params (Obstacle :type "CObstacle Object Reference"))
  (for _array_element (`self.ObstaclesSaved`)
    (if (== (break `/Game/Blueprints/GameTools/MapCreator/F_SaveData` _array_element) Obstacle)
      (`Actor.K2_SetActorLocation` (break `/Game/Blueprints/GameTools/MapCreator/F_SaveData` _array_element) (`Actor.K2_GetActorLocation` Obstacle) false false)
      (`Actor.K2_SetActorRotation` (break `/Game/Blueprints/GameTools/MapCreator/F_SaveData` _array_element) (`Actor.K2_GetActorRotation` Obstacle) false))))

(fn `GetIsCreatorMap`
  (returns (bIsCreatorMap :type Boolean))
  (return (`self.bIsCreatorMap`)))

(fn `GetSaveData`
  (returns (SaveData :type "Array of /Game/Blueprints/GameTools/MapCreator/F_SaveData Structure"))
  (return (`self.ObstaclesSaved`)))