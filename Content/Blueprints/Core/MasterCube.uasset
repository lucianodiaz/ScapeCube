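; MasterCube is a cube actor that colors itself blue and exposes that color to other code.
; On BeginPlay it converts a fixed blue color to a vector, stores it in ColorCube and applies it to the mesh materials' Color parameter.
; GetColorCube returns the stored vector, while the overlap, Tick and construction graphs are empty.
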(event `self.ReceiveBeginPlay`
  (bind (_color_b _color_g _color_r) (break `Color` (make `Color` 1 0 0 1)))
  (bind _output_get (set `self.ColorCube` (`KismetMathLibrary.MakeVector` (`KismetMathLibrary.Conv_ByteToDouble` _color_r) (`KismetMathLibrary.Conv_ByteToDouble` _color_g) (`KismetMathLibrary.Conv_ByteToDouble` _color_b))))
  (`MeshComponent.SetVectorParameterValueOnMaterials` (`self.MeshComponent`) "Color" _output_get))

(event `self.ReceiveTick`
  (params (DeltaSeconds :type "Float (single-precision)")))

(fn `GetColorCube`
  (returns (Color :type "Vector Structure"))
  (return (`self.ColorCube`)))

(fn `UserConstructionScript`)